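; Procedural product display area that fills a sized volume with rows of product meshes, one section per mesh.
; Construction measures mesh bounds, then layout splits the width evenly and derives width, depth and height counts from product size and gap.
; Each section is a spawned BP_ProductAreaSection that starts its own gradual generation.
; Sections spawn all at once or one per looping timer tick, which reports step and completion.
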(event `self.ReceiveBeginPlay`
  (if (`self.ShouldGenerateImmediately`)
    (`self.GenerateImmediately`)))

(fn `CalculateLayout`
  (locals (SectionWidthStandard :type "Float (double-precision)") (FilledSpace :type "Float (double-precision)"))
  (bind _size_x (`KismetMathLibrary.BreakVector` (`self.Size`)))
  (bind _size_x_2 (`KismetMathLibrary.BreakVector` (`self.Size`)))
  (bind (_size_x_3 _size_y _size_z) (`KismetMathLibrary.BreakVector` (`self.Size`)))
  (`KismetArrayLibrary.Array_Clear` (`self.SectionWidthCounts`))
  (`KismetArrayLibrary.Array_Clear` (`self.SectionDepthCounts`))
  (`KismetArrayLibrary.Array_Clear` (`self.SectionHeightCounts`))
  (set `local.FilledSpace` 0.0)
  (set `local.SectionWidthStandard` (/ _size_x (`KismetMathLibrary.Conv_IntToDouble` (`KismetArrayLibrary.Array_Length` (`self.Meshes`)))))
  (for _array_element (`self.ProductSizes`)
    (`|ExecutionSequence`
      (:`then_0`
        (bind _returnvalue (+ (.x _array_element) (`self.ObjectGap`)))
        (bind _returnvalue_2 (`KismetMathLibrary.FFloor` (/ (`local.SectionWidthStandard`) _returnvalue)))
        (bind _returnvalue_3 (* _returnvalue (`KismetMathLibrary.Conv_IntToDouble` _returnvalue_2)))
        (bind _output_get (set `local.FilledSpace` (+ _returnvalue_3 (`local.FilledSpace`))))
        (`KismetArrayLibrary.Array_Add` (`self.SectionWidthCounts`) (`KismetMathLibrary.SelectInt` _returnvalue_2 (`KismetMathLibrary.FTrunc` (/ (`KismetMathLibrary.SelectFloat` (- _size_x_2 _output_get) _returnvalue_3) _returnvalue)))))
      (:`then_1`
        (`KismetArrayLibrary.Array_Add` (`self.SectionDepthCounts`) (`KismetMathLibrary.FTrunc` (/ _size_y (+ (.y _array_element) (`self.ObjectGap`))))))
      (:`then_2`
        (`KismetArrayLibrary.Array_Add` (`self.SectionHeightCounts`) (`KismetMathLibrary.Max` (`KismetMathLibrary.FTrunc` (/ _size_z (.z _array_element))) 1))))))

(fn `CheckGradualGenerateComplete`
  (if (`self.IsGraduallyGenerating`)
    (bind _output_get (set `self.IsGraduallyGenerating` (<= (`self.CurrentGradualGenerateIndex`) (`self.SectionCount`))))
    (if (not _output_get)
      (`KismetSystemLibrary.K2_ClearTimer` null "GradualGenerateStep")
      (`self.GenerationComplete`))))

(fn `ClearAllPlacedInstances`
  (bind _sections (`self.Sections`))
  (for _array_element _sections
    (`/Game/GMUE4_ProcGen/blueprints/BP_ProductAreaSection.ClearAllPlacedInstances` _array_element)
    (`self.K2_DestroyActor` _array_element))
  (`KismetArrayLibrary.Array_Clear` _sections))

(fn `GenerateImmediately`
  (`self.ClearAllPlacedInstances`)
  (`self.CalculateLayout`)
  (for (_ _array_index) (`self.Meshes`)
    (`self.GenerateSection` _array_index)))

(fn `GenerateSection`
  (params (Index :type Integer))
  (locals (CurrentSectionStartX :type "Float (double-precision)"))
  (bind (_size_x _size_y) (`KismetMathLibrary.BreakVector` (`self.Size`)))
  (bind _flipped (`self.Flipped`))
  (set `local.CurrentSectionStartX` 0.0)
  (for (_array_element _array_index) (`self.SectionWidthCounts`)
    (if (< _array_index Index)
      (bind _output_x (`KismetMathLibrary.BreakVector` (`|GetArrayItem` (`self.ProductSizes`) _array_index)))
      (set `local.CurrentSectionStartX` (+ (`local.CurrentSectionStartX`) (* _array_element (+ (`self.ObjectGap`) _output_x))))
      (else
        (break))))
  (bind _returnvalue (`|SpawnActorFromClass` "/Game/GMUE4_ProcGen/blueprints/BP_ProductAreaSection.BP_ProductAreaSection_C" (`SceneComponent.GetRelativeTransform` (`self.DefaultSceneRoot`)) "Undefined" "OverrideRootScale" null (`self.ObjectGap`) (`self.Variance`) (- (`|GetArrayItem` (`self.SectionWidthCounts`) Index) 1) (- (`|GetArrayItem` (`self.SectionDepthCounts`) Index) 1) (- (`|GetArrayItem` (`self.SectionHeightCounts`) Index) 1) (`KismetMathLibrary.MakeVector` (`local.CurrentSectionStartX`) (`KismetMathLibrary.SelectFloat` _size_y 0.0 (not _flipped))) _flipped (`|GetArrayItem` (`self.ProductMeshes`) Index) (`|GetArrayItem` (`self.ProductSizes`) Index) (`self.ShouldGenerateImmediately`) 0.5 null))
  (`KismetArrayLibrary.Array_Add` (`self.Sections`) _returnvalue)
  (`/Game/GMUE4_ProcGen/blueprints/BP_ProductAreaSection.StartGradualGenerate` _returnvalue))

(fn `GradualGenerateStep`
  (bind _currentgradualgenerateindex (`self.CurrentGradualGenerateIndex`))
  (`self.GenerateSection` _currentgradualgenerateindex)
  (`self.GenerationStep` _currentgradualgenerateindex (`self.SectionCount`))
  (set `self.CurrentGradualGenerateIndex` (+ (`self.CurrentGradualGenerateIndex`) 1))
  (`self.CheckGradualGenerateComplete`))

(fn `InitMesh`
  (params (Mesh :type "StaticMesh Object Reference"))
  (returns (Instance :type "InstancedStaticMeshComponent Object Reference") (Size :type "Vector Structure"))
  (bind _returnvalue (`AddComponent|NODE_AddInstancedStaticMeshComponent-0`))
  (`StaticMeshComponent.SetStaticMesh` _returnvalue Mesh)
  (bind _size (`self.MeasureMesh` Mesh))
  (return _returnvalue _size))

(fn `MeasureMesh`
  (params (mesh :type "StaticMesh Object Reference"))
  (returns (size :type "Vector Structure"))
  (locals (MeshSize :type "Vector Structure"))
  (bind (_min _max) (break `Box` (`StaticMesh.GetBoundingBox` mesh)))
  (bind _returnvalue (`AddComponent|NODE_AddStaticMeshComponent-0`))
  (`StaticMeshComponent.SetStaticMesh` _returnvalue mesh)
  (bind _output_get (set `local.MeshSize` (- _max _min)))
  (`ActorComponent.K2_DestroyComponent` _returnvalue)
  (return _output_get))

(fn `StartGradualGenerate`
  (if (not (`self.IsGraduallyGenerating`))
    (`self.ClearAllPlacedInstances`)
    (`self.CalculateLayout`)
    (set `self.CurrentGradualGenerateIndex` 0)
    (set `self.IsGraduallyGenerating` true)
    (bind _returnvalue (`KismetSystemLibrary.K2_SetTimer` null "GradualGenerateStep" (`self.GenerateInterval`) true (`self.GenerateStartDelay`)))
    (set `self.GenerationLoopHandle` _returnvalue)))

(fn `UserConstructionScript`
  (bind _productmeshes (`self.ProductMeshes`))
  (`|ExecutionSequence`
    (:`then_0`
      (for _array_element _productmeshes
        (bind (_instance _size) (`self.InitMesh` _array_element))
        (`KismetArrayLibrary.Array_Add` (`self.Meshes`) _instance)
        (`KismetArrayLibrary.Array_Add` (`self.ProductSizes`) _size))
      (set `self.SectionCount` (- (`KismetArrayLibrary.Array_Length` _productmeshes) 1)))
    (:`then_1`
      (`self.ClearAllPlacedInstances`)
      (`self.CalculateLayout`)
      (if (`self.ShouldGenerateImmediately`)
        (`self.GenerateImmediately`)))))