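; BP_ProductAreaSection fills a section with a 3D grid of one mesh as instances, apparently representing stocked products.
; The construction script creates the instanced mesh component and can fill the whole grid immediately.
; GenerateXStep places one width slice, jittering position and yaw by Variance and optionally flipping Y.
; StartGradualGenerate clears instances, then a looping timer adds slices, calling step and completion notifications.
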(fn `CheckGradualGenerateComplete`
  (if (`self.IsGraduallyGenerating`)
    (bind _output_get (set `self.IsGraduallyGenerating` (< (`self.CurrentGradualGenerateIndex`) (`self.WidthCount`))))
    (if (not _output_get)
      (`KismetSystemLibrary.K2_ClearTimer` null "GradualGenerateStep")
      (`self.GenerationComplete`))))

(fn `ClearAllPlacedInstances`
  (`InstancedStaticMeshComponent.ClearInstances` (`self.Instance`)))

(fn `GenerateImmediately`
  (for _index (range (+ (`self.WidthCount`) 1))
    (`self.GenerateXStep` _index)))

(fn `GenerateXStep`
  (params (Index :type Integer))
  (bind (_instancearea_x _instancearea_y) (`KismetMathLibrary.BreakVector` (`self.InstanceArea`)))
  (bind _instancesize_x (`KismetMathLibrary.BreakVector` (`self.InstanceSize`)))
  (bind (_instancesize_x_2 _instancesize_y _instancesize_z) (`KismetMathLibrary.BreakVector` (`self.InstanceSize`)))
  (bind _returnvalue (* (/ (`self.ObjectGap`) 2.0) (`self.Variance`)))
  (bind _returnvalue_2 (* _returnvalue -1.0))
  (for _index (range (+ (`self.DepthCount`) 1))
    (for _index_2 (range (+ (`self.HeightCount`) 1))
      (bind _returnvalue_3 (+ (* _index _instancearea_y) (/ _instancesize_y 2.0)))
      (`InstancedStaticMeshComponent.AddInstance` (`self.Instance`) (`KismetMathLibrary.MakeTransform` (+ (+ (`KismetMathLibrary.MakeVector` (+ (* Index _instancearea_x) (/ _instancesize_x_2 2.0)) (`KismetMathLibrary.SelectFloat` (* _returnvalue_3 -1.0) _returnvalue_3 (not (`self.Flipped`))) (* _index_2 _instancesize_z)) (`KismetMathLibrary.MakeVector` (`KismetMathLibrary.RandomFloatInRange` _returnvalue_2 _returnvalue) (`KismetMathLibrary.RandomFloatInRange` _returnvalue_2 _returnvalue))) (`self.OriginLocation`) (`KismetMathLibrary.MakeVector` (/ _instancesize_x 2.0))) (`KismetMathLibrary.MakeRotator` 0.0 0.0 (`KismetMathLibrary.RandomFloatInRange` (* _returnvalue -3.0) (* _returnvalue 3.0))))))))

(fn `GradualGenerateStep`
  (bind _currentgradualgenerateindex (`self.CurrentGradualGenerateIndex`))
  (`self.GenerateXStep` _currentgradualgenerateindex)
  (`self.GenerationStep` _currentgradualgenerateindex (`self.WidthCount`))
  (set `self.CurrentGradualGenerateIndex` (+ (`self.CurrentGradualGenerateIndex`) 1))
  (`self.CheckGradualGenerateComplete`))

(fn `StartGradualGenerate`
  (if (not (`self.IsGraduallyGenerating`))
    (`self.ClearAllPlacedInstances`)
    (set `self.CurrentGradualGenerateIndex` 0)
    (set `self.IsGraduallyGenerating` true)
    (bind _returnvalue (`KismetSystemLibrary.K2_SetTimer` null "GradualGenerateStep" (`self.GenerateInterval`) true (`self.GenerateStartDelay`)))
    (set `self.GenerateLoopHandle` _returnvalue)))

(fn `UserConstructionScript`
  (bind (_instancesize_x _instancesize_y _instancesize_z) (`KismetMathLibrary.BreakVector` (`self.InstanceSize`)))
  (bind _objectgap (`self.ObjectGap`))
  (set `self.InstanceArea` (`KismetMathLibrary.MakeVector` (+ _instancesize_x _objectgap) (+ _instancesize_y _objectgap) _instancesize_z))
  (bind _returnvalue (`AddComponent|NODE_AddInstancedStaticMeshComponent-0`))
  (`StaticMeshComponent.SetStaticMesh` _returnvalue (`self.Mesh`))
  (set `self.Instance` _returnvalue)
  (if (`self.ShouldGenerateImmediately`)
    (`self.GenerateImmediately`)))