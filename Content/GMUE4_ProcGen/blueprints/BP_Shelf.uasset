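; BP_Shelf is a procedural shelving run that builds start, middle and end sections as instanced static meshes along X.
; Construction creates the components, measures mesh bounds for spacing and optionally generates every section at once.
; A looping timer offers gradual generation, and both modes fire step and completion dispatchers.
; A Flipped flag mirrors placement, and size helpers derive per-height product areas from the mesh measurements.
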(fn `CheckGradualGenerateComplete`
  (if (`self.IsGraduallyGenerating`)
    (bind _output_get (set `self.IsGraduallyGenerating` (<= (`self.CurrentGradualGenerateIndex`) (`self.UsedLength`))))
    (if (not _output_get)
      (`KismetSystemLibrary.K2_ClearTimer` null "GradualGenerateStep")
      (`self.GenerationComplete`))))

(fn `ClearAllPlacedInstancesAndMeshes`
  (`InstancedStaticMeshComponent.ClearInstances` (`self.Shelf`))
  (`InstancedStaticMeshComponent.ClearInstances` (`self.ShelfStart`))
  (`InstancedStaticMeshComponent.ClearInstances` (`self.ShelfEnd`)))

(fn `GenerateImmediately`
  (bind _usedlength (`self.UsedLength`))
  (for _index (range (+ _usedlength 1))
    (`self.GenerateShelfSection` _index)
    (`self.GenerationStep` _index _usedlength))
  (`self.GenerationComplete`))

(fn `GenerateShelfSection`
  (params (Index :type Integer))
  (locals (IndexInUse :type Integer))
  (bind _flipped (`self.Flipped`))
  (bind _indexinuse (`local.IndexInUse`))
  (bind _shelfsize_x (`KismetMathLibrary.BreakVector` (`self.ShelfSize`)))
  (bind _shelfstartsize_x (`KismetMathLibrary.BreakVector` (`self.ShelfStartSize`)))
  (bind _shelfstartsize_x_2 (`KismetMathLibrary.BreakVector` (`self.ShelfStartSize`)))
  (bind _shelfsize_x_2 (`KismetMathLibrary.BreakVector` (`self.ShelfSize`)))
  (bind _flipped_2 (`self.Flipped`))
  (bind _returnvalue (`KismetMathLibrary.SelectFloat` 180.0 0.0 _flipped))
  (bind _returnvalue_2 (- _shelfsize_x 3.0))
  (bind _returnvalue_3 (`KismetMathLibrary.MakeTransform` (`KismetMathLibrary.MakeVector` (+ (* (- (`local.IndexInUse`) 1) _returnvalue_2) (`KismetMathLibrary.SelectFloat` (+ _returnvalue_2 _shelfstartsize_x_2) _shelfstartsize_x_2 _flipped_2) (`KismetMathLibrary.SelectFloat` -6.0 0.0 _flipped_2))) (`KismetMathLibrary.MakeRotator` 0.0 0.0 _returnvalue)))
  (set `local.IndexInUse` (`KismetMathLibrary.SelectInt` (- (`self.UsedLength`) Index) Index _flipped))
  (if (== _indexinuse (`KismetMathLibrary.SelectInt` (`self.UsedLength`) 0 _flipped))
    (`InstancedStaticMeshComponent.AddInstance` (`self.ShelfStart`) (`KismetMathLibrary.MakeTransform` (`KismetMathLibrary.MakeVector` (`KismetMathLibrary.SelectFloat` (+ (* (`self.UsedLength`) (- _shelfsize_x_2 3.0)) _shelfstartsize_x) 0.0 (`self.Flipped`))) (`KismetMathLibrary.MakeRotator` 0.0 0.0 _returnvalue)))
    (elif (== _indexinuse (`KismetMathLibrary.SelectInt` 0 (`self.UsedLength`) (`self.Flipped`)))
      (`InstancedStaticMeshComponent.AddInstance` (`self.ShelfEnd`) _returnvalue_3)
      (else
        (`InstancedStaticMeshComponent.AddInstance` (`self.Shelf`) _returnvalue_3)))))

(fn `GetProductAreas`
  (returns (ProductAreas :type "Array of /Game/GMUE4_ProcGen/blueprints/SShelfAreaDefinition Structure"))
  (locals (Areas :type "Array of /Game/GMUE4_ProcGen/blueprints/SShelfAreaDefinition Structure"))
  (bind _returnvalue (`SceneComponent.GetRelativeTransform` (`self.DefaultSceneRoot`)))
  (bind (_size _shelfzlocations) (`self.GetSize`))
  (for _array_element _shelfzlocations
    (`KismetArrayLibrary.Array_Add` (`local.Areas`) (make `/Game/GMUE4_ProcGen/blueprints/SShelfAreaDefinition` (`KismetMathLibrary.MakeTransform` (`KismetMathLibrary.MakeVector` (.x (.location _returnvalue)) (+ (.y (.location _returnvalue)) (`KismetMathLibrary.SelectFloat` 0.0 (`self.ShelfBackDepth`) (`self.Flipped`))) (+ (.z (.location _returnvalue)) _array_element)) (.rotation _returnvalue) (.scale _returnvalue)) (`KismetMathLibrary.MakeVector` (.x _size) (.y _size) (`self.ShelfUsableGap`)) (`self.Flipped`))))
  (return))

(fn `GetSize`
  (returns (Size :type "Vector Structure") (ShelfZLocations :type "Array of Float (double-precision)"))
  (locals (Areas :type "Array of /Game/GMUE4_ProcGen/blueprints/SShelfAreaDefinition Structure"))
  (bind _shelfendsize_x (`KismetMathLibrary.BreakVector` (`self.ShelfEndSize`)))
  (bind (_shelfsize_x _shelfsize_y _shelfsize_z) (`KismetMathLibrary.BreakVector` (`self.ShelfSize`)))
  (bind _shelfstartsize_x (`KismetMathLibrary.BreakVector` (`self.ShelfStartSize`)))
  (return (`KismetMathLibrary.MakeVector` (+ (* (- _shelfsize_x 1.0) (`KismetMathLibrary.Conv_IntToDouble` (- (`self.Length`) 2))) _shelfstartsize_x _shelfendsize_x) (- _shelfsize_y (`self.ShelfBackDepth`)) _shelfsize_z) (`self.InnerShelfHeights`)))

(fn `GradualGenerateStep`
  (bind _currentgradualgenerateindex (`self.CurrentGradualGenerateIndex`))
  (`self.GenerateShelfSection` _currentgradualgenerateindex)
  (`self.GenerationStep` _currentgradualgenerateindex (`self.UsedLength`))
  (set `self.CurrentGradualGenerateIndex` (+ (`self.CurrentGradualGenerateIndex`) 1))
  (`self.CheckGradualGenerateComplete`))

(fn `InitMesh`
  (params (Mesh :type "StaticMesh Object Reference"))
  (returns (Instance :type "InstancedStaticMeshComponent Object Reference") (Size :type "Vector Structure"))
  (bind _returnvalue (`AddComponent|NODE_AddInstancedStaticMeshComponent-1`))
  (`StaticMeshComponent.SetStaticMesh` _returnvalue Mesh)
  (bind _size (`self.MeasureMesh` Mesh))
  (return _returnvalue _size))

(fn `MeasureMesh`
  (params (Mesh :type "StaticMesh Object Reference"))
  (returns (Size :type "Vector Structure"))
  (locals (MeshSize :type "Vector Structure"))
  (bind (_min _max) (break `Box` (`StaticMesh.GetBoundingBox` Mesh)))
  (bind _returnvalue (`AddComponent|NODE_AddStaticMeshComponent-0`))
  (`StaticMeshComponent.SetStaticMesh` _returnvalue Mesh)
  (bind _output_get (set `local.MeshSize` (- _max _min)))
  (`ActorComponent.K2_DestroyComponent` _returnvalue)
  (return _output_get))

(fn `StartGradualGenerate`
  (set `self.CurrentGradualGenerateIndex` 0)
  (set `self.IsGraduallyGenerating` true)
  (bind _returnvalue (`KismetSystemLibrary.K2_SetTimer` null "GradualGenerateStep" (`self.GenerateInterval`) true 0.0 (`self.GenerateStartDelay`)))
  (set `self.GenerateLoopHandle` _returnvalue))

(fn `UserConstructionScript`
  (`|ExecutionSequence`
    (:`then_0`
      (bind (_instance _size) (`self.InitMesh` (`self.ShelfMesh`)))
      (set `self.Shelf` _instance)
      (set `self.ShelfSize` _size)
      (bind (_instance_2 _size_2) (`self.InitMesh` (`self.ShelfStartMesh`)))
      (set `self.ShelfStart` _instance_2)
      (set `self.ShelfStartSize` _size_2)
      (bind (_instance_3 _size_3) (`self.InitMesh` (`self.ShelfEndMesh`)))
      (set `self.ShelfEnd` _instance_3)
      (set `self.ShelfEndSize` _size_3))
    (:`then_1`
      (set `self.UsedLength` (- (`self.Length`) 1)))
    (:`then_2`
      (`self.ClearAllPlacedInstancesAndMeshes`)
      (if (`self.ShouldGenerateImmediately`)
        (`self.GenerateImmediately`)))))