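; Procedural store aisle generator that spawns rows of BP_Shelf actors, sized from XSize and YSize and spaced by AisleWidth.
; Alternate shelves are flipped and paired at shared offsets, with their product areas collected into one list.
; The construction script rebuilds immediately, while RegenerateAtSize clears and respawns shelves gradually on a looping timer.
; Both paths call GenerationStep per shelf and GenerationComplete at the end.
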(event `self.ReceiveBeginPlay`
  (`self.CalculateGenerateCounts`))

(fn `CalculateGenerateCounts`
  (set `self.ShelfCount` (- (* (`self.YSize`) 2) 1))
  (set `self.ShelfLength` (- (* (`self.XSize`) 2) 1)))

(fn `CheckGradualGenerateComplete`
  (if (`self.IsGraduallyGenerating`)
    (bind _output_get (set `self.IsGraduallyGenerating` (<= (`self.CurrentGradualGenerateIndex`) (`self.ShelfCount`))))
    (if (not _output_get)
      (`KismetSystemLibrary.K2_ClearTimer` null "GradualGenerateStep")
      (`self.GenerationComplete`))))

(fn `ClearAllGenerated`
  (bind _spawnedshelflist (`self.SpawnedShelfList`))
  (for _array_element _spawnedshelflist
    (`self.K2_DestroyActor` _array_element))
  (`KismetArrayLibrary.Array_Clear` _spawnedshelflist)
  (`KismetArrayLibrary.Array_Clear` (`self.ProductAreas`)))

(fn `GenerateImmediately`
  (bind _returnvalue (- (`self.ShelfCount`) 1))
  (for _index (range (+ _returnvalue 1))
    (bind (_latestshelf _shelfproductareas) (`self.GenerateShelf` _index true))
    (`self.GenerationStep` _index _returnvalue _shelfproductareas))
  (`self.GenerationComplete`))

(fn `GenerateShelf`
  (params (Index :type Integer) (ShouldGenerateImmediately :type Boolean :default false))
  (returns (LatestShelf :type "/Game/GMUE4_ProcGen/blueprints/BP_Shelf Object Reference") (ShelfProductAreas :type "Array of /Game/GMUE4_ProcGen/blueprints/SShelfAreaDefinition Structure"))
  (bind _returnvalue (`SceneComponent.GetRelativeTransform` (`self.DefaultSceneRoot`)))
  (bind _returnvalue_2 (`|SpawnActorFromClass` "/Game/GMUE4_ProcGen/blueprints/BP_Shelf.BP_Shelf_C" (`KismetMathLibrary.MakeTransform` (`KismetMathLibrary.MakeVector` (+ (.x (.location _returnvalue)) 200.0) (+ (`KismetMathLibrary.Conv_IntToDouble` (* (/ (+ Index 1) 2) (`self.AisleWidth`))) (.y (.location _returnvalue)) 0.0) (.z (.location _returnvalue))) (.rotation _returnvalue)) "Undefined" "OverrideRootScale" null (`self.ShelfLength`) (!= (mod Index 2) 0) ShouldGenerateImmediately 0.05 0.0 null))
  (`KismetArrayLibrary.Array_Add` (`self.SpawnedShelfList`) _returnvalue_2)
  (bind _productareas (`/Game/GMUE4_ProcGen/blueprints/BP_Shelf.GetProductAreas` _returnvalue_2))
  (`KismetArrayLibrary.Array_Append` (`self.ProductAreas`) _productareas)
  (`/Game/GMUE4_ProcGen/blueprints/BP_Shelf.StartGradualGenerate` _returnvalue_2)
  (return _returnvalue_2 _productareas))

(fn `GradualGenerateStep`
  (bind _currentgradualgenerateindex (`self.CurrentGradualGenerateIndex`))
  (bind (_latestshelf _shelfproductareas) (`self.GenerateShelf` _currentgradualgenerateindex))
  (`self.GenerationStep` _currentgradualgenerateindex (- (`self.ShelfCount`) 1) _shelfproductareas)
  (set `self.CurrentGradualGenerateIndex` (+ (`self.CurrentGradualGenerateIndex`) 1))
  (`self.CheckGradualGenerateComplete`))

(fn `RegenerateAtSize`
  (params (XSize :type Integer) (YSize :type Integer) (AisleWidth :type Integer))
  (if (not (`self.IsGraduallyGenerating`))
    (set `self.XSize` XSize)
    (set `self.YSize` YSize)
    (set `self.AisleWidth` AisleWidth)
    (`self.CalculateGenerateCounts`)
    (`self.StartGradualGenerate`)))

(fn `StartGradualGenerate`
  (if (not (`self.IsGraduallyGenerating`))
    (`self.ClearAllGenerated`)
    (set `self.CurrentGradualGenerateIndex` 0)
    (set `self.IsGraduallyGenerating` true)
    (bind _returnvalue (`KismetSystemLibrary.K2_SetTimer` null "GradualGenerateStep" (`self.GenerateInterval`) true (`self.GenerateDelay`)))
    (set `self.GenerateLoopHandle` _returnvalue)))

(fn `UserConstructionScript`
  (`self.ClearAllGenerated`)
  (`self.CalculateGenerateCounts`)
  (`self.GenerateImmediately`))