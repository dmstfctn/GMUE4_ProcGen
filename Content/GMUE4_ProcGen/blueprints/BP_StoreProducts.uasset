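; BP_StoreProducts populates store areas with procedurally placed products by spawning and tracking BP_ProductArea actors.
; AddProductsFromAreas gives each area a shuffled random subset of product meshes with random gap and variance, while RegenerateFromAreas uses fixed spacing and index-staggered start delays.
; Both offset transforms along Y according to each area's flip flag and start gradual generation.
; ClearAllGenerated clears placed instances and destroys the tracked actors.
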(fn `AddProductsFromAreas`
  (params (Areas :type "Array of /Game/GMUE4_ProcGen/blueprints/SShelfAreaDefinition Structure"))
  (locals (ProductsForArea :type "Array of StaticMesh Object Reference"))
  (bind _allproducts (`self.AllProducts`))
  (bind _returnvalue (`KismetArrayLibrary.Array_Length` _allproducts))
  (bind _returnvalue_2 (`KismetMathLibrary.RandomIntegerInRange` (`KismetMathLibrary.Min` 3 _returnvalue) (`KismetMathLibrary.Min` 15 _returnvalue)))
  (`KismetArrayLibrary.Array_Append` (`self.Areas`) Areas)
  (for _array_element Areas
    (`KismetArrayLibrary.Array_Clear` (`local.ProductsForArea`))
    (`KismetArrayLibrary.Array_Shuffle` _allproducts)
    (`KismetSystemLibrary.PrintString` (`KismetStringLibrary.BuildString_Int` "" "product type count: " _returnvalue_2))
    (for _index (range (+ _returnvalue_2 1))
      (`KismetArrayLibrary.Array_AddUnique` (`local.ProductsForArea`) (`|GetArrayItem` (`self.AllProducts`) _index)))
    (bind _transformresult (`self.CalculateProductAreaTransform` (break `/Game/GMUE4_ProcGen/blueprints/SShelfAreaDefinition` _array_element) (`.Size_5_91793C7742477457B4A6AA851D894C83` (break `/Game/GMUE4_ProcGen/blueprints/SShelfAreaDefinition` _array_element)) (`.IsFlippedOnY_8_36465EED467F5992D150888A4A7F03A6` (break `/Game/GMUE4_ProcGen/blueprints/SShelfAreaDefinition` _array_element))))
    (bind _returnvalue_3 (`|SpawnActorFromClass` "/Game/GMUE4_ProcGen/blueprints/BP_ProductArea.BP_ProductArea_C" _transformresult "Undefined" "OverrideRootScale" null (`.Size_5_91793C7742477457B4A6AA851D894C83` (break `/Game/GMUE4_ProcGen/blueprints/SShelfAreaDefinition` _array_element)) (`KismetMathLibrary.RandomFloatInRange` 1.0 4.0) (`KismetMathLibrary.RandomFloatInRange` 0.1 1.0) false (`local.ProductsForArea`) false 0.3 0.0 null))
    (`KismetArrayLibrary.Array_Add` (`self.GeneratedProductAreas`) _returnvalue_3)
    (`/Game/GMUE4_ProcGen/blueprints/BP_ProductArea.StartGradualGenerate` _returnvalue_3)))

(fn `CalculateProductAreaTransform`
  (params (InitialTransform :type "Transform Structure") (Size :type "Vector Structure") (IsFlipped :type Boolean))
  (returns (TransformResult :type "Transform Structure"))
  (locals (ProductsForArea :type "Array of StaticMesh Object Reference"))
  (return (`KismetMathLibrary.MakeTransform` (`KismetMathLibrary.MakeVector` (.x (.location InitialTransform)) (`KismetMathLibrary.SelectFloat` (- (.y (.location InitialTransform)) Size_Y) (.y (.location InitialTransform)) IsFlipped) (.z (.location InitialTransform))) InitialTransform_Rotation InitialTransform_Scale)))

(fn `ClearAllGenerated`
  (bind _generatedproductareas (`self.GeneratedProductAreas`))
  (for _array_element _generatedproductareas
    (`/Game/GMUE4_ProcGen/blueprints/BP_ProductArea.ClearAllPlacedInstances` _array_element)
    (`self.K2_DestroyActor` _array_element))
  (`KismetArrayLibrary.Array_Clear` _generatedproductareas))

(fn `RegenerateFromAreas`
  (params (Areas :type "Array of /Game/GMUE4_ProcGen/blueprints/SShelfAreaDefinition Structure"))
  (bind _output_get (set `self.Areas` Areas))
  (for (_array_element _array_index) _output_get
    (bind _transformresult (`self.CalculateProductAreaTransform` (break `/Game/GMUE4_ProcGen/blueprints/SShelfAreaDefinition` _array_element) (`.Size_5_91793C7742477457B4A6AA851D894C83` (break `/Game/GMUE4_ProcGen/blueprints/SShelfAreaDefinition` _array_element)) (`.IsFlippedOnY_8_36465EED467F5992D150888A4A7F03A6` (break `/Game/GMUE4_ProcGen/blueprints/SShelfAreaDefinition` _array_element))))
    (bind _returnvalue (`|SpawnActorFromClass` :`Class` "/Game/GMUE4_ProcGen/blueprints/BP_ProductArea.BP_ProductArea_C" :`SpawnTransform` _transformresult :`CollisionHandlingOverride` "Undefined" :`TransformScaleMethod` "OverrideRootScale" :`Size` (`.Size_5_91793C7742477457B4A6AA851D894C83` (break `/Game/GMUE4_ProcGen/blueprints/SShelfAreaDefinition` _array_element)) :`ObjectGap` 1.0 :`GenerateInterval` 1.0 :`GenerateStartDelay` (`KismetMathLibrary.Conv_IntToDouble` _array_index) :`Instigator` null))
    (`KismetArrayLibrary.Array_Add` (`self.GeneratedProductAreas`) _returnvalue)
    (`/Game/GMUE4_ProcGen/blueprints/BP_ProductArea.StartGradualGenerate` _returnvalue)))

(fn `UserConstructionScript`)